(event `Write`
  (bind _parent_component (`self.Parent Component`))
  (`KismetSystemLibrary.Delay` 0.05)
  (bind _returnvalue (`|SpawnActorFromClass` "/Game/LowPolyText/Blueprints/LowPolyTextActor.LowPolyTextActor_C" (`SceneComponent.K2_GetComponentToWorld` (`self.ParentMeshRef`)) "AlwaysSpawn" "OverrideRootScale" null (`self.Text Data`)))
  (bind _output_get (set `self.LowPoly Text Actor` _returnvalue))
  (`|ExecutionSequence`
    (:`then_0`
      (`/Engine/EditorBlueprintResources/StandardMacros.IsValid` _output_get))
    (:`then_1`
      (`/Engine/EditorBlueprintResources/StandardMacros.IsValid` _parent_component
        (:`Is Valid`
          (`Actor.K2_AttachToComponent` _output_get _parent_component "None" "KeepWorld" "KeepWorld" "KeepWorld" true))
        (:`Is Not Valid`
          (`Actor.K2_AttachToActor` _output_get (`self.GetOwner`) "None" "KeepWorld" "KeepWorld" "KeepWorld" true))))))

(event `Erase`
  (`/Game/LowPolyText/Blueprints/LowPolyTextActor.Erase Text` (`self.LowPoly Text Actor`)))

(event `Destroy TExt`
  (bind _lowpoly_text_actor (`self.LowPoly Text Actor`))
  (`/Engine/EditorBlueprintResources/StandardMacros.IsValid` _lowpoly_text_actor
    (:`Is Valid`
      (`Actor.K2_DestroyActor` _lowpoly_text_actor))))