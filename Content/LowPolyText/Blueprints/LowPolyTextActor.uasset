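; Actor that displays multi-line text as 3D letter meshes, generated in the construction script and again on BeginPlay.
; GenerateText spawns a static mesh component per TextData character, spaced by character and line gaps.
; GetLetter looks up each character in Alphabet for mesh, displacement, rotation and scale, combined with line scale and per-character adjustments.
; Per-character materials fall back to the line material; EraseText destroys the tracked components.
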(event `self.ReceiveBeginPlay`
  (`self.Generate Text`))

(event `self.ReceiveTick`
  (params (DeltaSeconds :type "Float (single-precision)")))

(event `Generate Text`
  ;[1 1 1] Generate Text
  (for (_array_element _array_index) (`self.Text Data`)
    (bind (_linestring _linegap _linescale _charactergap _linematerial _characteroffests _characterscales _charactermaterials) (break `/Game/LowPolyText/DataStructs/TextData` _array_element))
    (for _index (range (+ (`KismetStringLibrary.Len` _linestring) 1))
      (bind (_mesh _newparam _newparam2 _newparam3) (`self.Get Letter` _index _array_index)
        (:`out`
          (bind _returnvalue (`AddComponent|NODE_AddStaticMeshComponent-0` :`RelativeTransform` (`KismetMathLibrary.MakeTransform` (+ _newparam (`KismetMathLibrary.MakeVector` (* _index _charactergap) (* _array_index _linegap)) (`KismetArrayLibrary.Array_Get` _characteroffests _index)) _newparam2 (+ (1.0 1.0 1.0) (+ _linescale _newparam3 (`KismetArrayLibrary.Array_Get` _characterscales _index))))))
          (`KismetArrayLibrary.Array_Add` (`self.Letter Array`) _returnvalue)
          (`StaticMeshComponent.SetStaticMesh` _returnvalue _mesh)
          (bind _item (`KismetArrayLibrary.Array_Get` _charactermaterials _index))
          (if (`KismetSystemLibrary.IsValid` _item)
            (`PrimitiveComponent.SetMaterial` _returnvalue 0 _item)
            (else
              (`PrimitiveComponent.SetMaterial` _returnvalue 0 _linematerial))))))))

(event `Erase Text`
  (bind _letter_array (`self.Letter Array`))
  ;[1 1 1] Generate Text
  (for _array_element _letter_array
    (`ActorComponent.K2_DestroyComponent` _array_element))
  (`KismetArrayLibrary.Array_Clear` _letter_array))

(fn `UserConstructionScript`
  (`self.Generate Text`))