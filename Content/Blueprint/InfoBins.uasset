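; InfoBins is an actor that shows a temporary text billboard when its ButtonPressed event fires.
; A press spawns a BillBoard at the actor's location if none is active, passing itself, height, text data and cable settings.
; Each press restarts a retriggerable delay, so the board stays for ten seconds after the last press.
; ClearBoard then erases the low-poly text, destroys the board and clears its reference.
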(event `/Game/Blueprint/ButtonInterface.Button Pressed`
  (params (`Button Index` :type Integer))
  (if (not (`KismetSystemLibrary.IsValid` (`self.Active Board`)))
    (`self.Spawn Board` self (`self.Height Offset`) (`self.Text Data`) (`self.Text Offest`)))
  (`KismetSystemLibrary.RetriggerableDelay` 10.0)
  (`self.Clear Board`))

(fn `Clear Board`
  (bind _active_board (`self.Active Board`))
  (`/Game/LowPolyText/Blueprints/LowPolyTextComp.Erase` (`/Game/Blueprint/BillBoard.LowPolyTextComp` _active_board))
  (`self.K2_DestroyActor` _active_board)
  (set `self.Active Board` null))

(fn `Spawn Board`
  (params (`Owning Actor` :type "Actor Object Reference") (`Height Offset` :type "Float (double-precision)") (`Text Data` :type "Array of /Game/LowPolyText/DataStructs/TextData Structure") (`Text Offset` :type "Vector Structure"))
  (bind _returnvalue (`|SpawnActorFromClass` "/Game/Blueprint/BillBoard.BillBoard_C" (`KismetMathLibrary.MakeTransform` (`self.K2_GetActorLocation` `Owning Actor`)) "Undefined" "OverrideRootScale" null 35.0 15.0 `Owning Actor` `Height Offset` `Text Data` `Text Offset`))
  (set `self.Active Board` _returnvalue))

(fn `UserConstructionScript`)