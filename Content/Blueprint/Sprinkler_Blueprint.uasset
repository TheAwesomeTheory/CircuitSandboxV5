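; Fire sprinkler Blueprint that sprays a particle effect with sound when its EmergencyHasHappened event is called.
; An On flag ignores repeat calls while a timed Delay sequence runs.
; After an initial delay it activates the particle system and plays the sprinkler sound twice at the actor's location.
; It then deactivates the particles and clears the flag, allowing it to trigger again.
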(event `/Game/Blueprint/Emergency.Emergency has happened`
  (params (NewParam :type Boolean))
  (if (not (`self.On`))
    (set `self.On` true)
    (`KismetSystemLibrary.Delay` 2.89)
    (`ActorComponent.Activate` (`self.ParticleSystem`) false)
    (`GameplayStatics.PlaySoundAtLocation` "/Game/Audio/firesprinkler.firesprinkler" (`self.K2_GetActorLocation`) (struct) 0.2)
    (`KismetSystemLibrary.Delay` 4.0)
    (`GameplayStatics.PlaySoundAtLocation` "/Game/Audio/firesprinkler.firesprinkler" (`self.K2_GetActorLocation`) (struct) 0.2)
    (`KismetSystemLibrary.Delay` 4.0)
    (`ActorComponent.Deactivate` (`self.ParticleSystem`))
    (`KismetSystemLibrary.Delay` 0.2)
    (set `self.On` false)))

(fn `UserConstructionScript`)