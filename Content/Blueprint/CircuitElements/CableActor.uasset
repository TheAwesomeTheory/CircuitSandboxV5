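; Cable actor that links two actors, attaching itself to the first and the cable component's end to the second at BeginPlay.
; Each tick, when their distance exceeds the cable length, it pulls physics-simulating CableCaps ends together with stiffness-scaled forces and resizes the visible cable to that distance minus an offset.
; The overstretch check is empty, and the velocity gate and detach logic are unwired.
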(event `self.ReceiveBeginPlay`
  (`self.K2_AttachToActor` (`self.Actor1`) "None" "SnapToTarget" "SnapToTarget" "KeepRelative")
  (`CableComponent.SetAttachEndTo` (`self.Cable`) (`self.Actor2`) "None" "None"))

(event `self.ReceiveTick`
  (params (DeltaSeconds :type "Float (single-precision)"))
  (bind _actor2 (`self.Actor2`))
  (bind _actor1 (`self.Actor1`))
  (bind _returnvalue (`KismetMathLibrary.VSize` (- (`self.K2_GetActorLocation` (`self.Actor2`)) (`self.K2_GetActorLocation` (`self.Actor1`)))))
  (if (< (`self.cablelength`) (`KismetMathLibrary.VSize` (- (`self.K2_GetActorLocation` (`self.Actor2`)) (`self.K2_GetActorLocation` (`self.Actor1`)))))
    (`|ExecutionSequence`
      (:`then_0`
        (bind _ascable_caps (cast `/Game/Blueprint/CircuitElements/CableCaps` _actor1))
        (if (`SceneComponent.IsSimulatingPhysics` (`StaticMeshActor.StaticMeshComponent` _ascable_caps) "None")
          (`PrimitiveComponent.AddForce` (`StaticMeshActor.StaticMeshComponent` _ascable_caps) (* (- (`self.K2_GetActorLocation` (`self.Actor2`)) (`self.K2_GetActorLocation` _actor1)) (`self.stiffness`)) "None" false)))
      (:`then_1`
        (if (< (* (`self.cablelength`) 2.0) _returnvalue)
          _))
      (:`then_2`
        (bind _ascable_caps_2 (cast `/Game/Blueprint/CircuitElements/CableCaps` _actor2))
        (if (`SceneComponent.IsSimulatingPhysics` (`StaticMeshActor.StaticMeshComponent` _ascable_caps_2) "None")
          (`PrimitiveComponent.AddForce` (`StaticMeshActor.StaticMeshComponent` _ascable_caps_2) (* (- (`self.K2_GetActorLocation` (`self.Actor1`)) (`self.K2_GetActorLocation` _actor2)) (`self.stiffness`)) "None" false)))
      (:`then_3`
        (set `CableComponent.CableLength` (- _returnvalue (`self.NewVar_0`)) (`self.Cable`))))))

(fn `UserConstructionScript`)