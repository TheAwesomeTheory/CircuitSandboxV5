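; Grabbable power supply for a VR circuit-building game, with motion-controller buttons that step voltage within limits.
; Terminal overlaps snap cable caps on and release them with a pop.
; Tick messages the caps, sending current through the positive one when closed, while PassCurrent derives current from returned resistance.
; A retriggerable delay reopens the circuit when PassCurrent stops arriving; voltage-text and button-press feedback logic is unwired.
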(event `self.ReceiveBeginPlay`)

(event `/Game/Blueprint/PickupActorInterface.Pickup`
  (params (AttachTo :type "SceneComponent Object Reference") (GrabbedComponent :type "SceneComponent Object Reference"))
  (`PrimitiveComponent.SetSimulatePhysics` (`self.StaticMeshComponent`) false)
  (`SceneComponent.K2_AttachToComponent` (`self.K2_GetRootComponent`) AttachTo "None" "KeepWorld" "KeepWorld" "KeepWorld" false))

(event `/Game/Blueprint/PickupActorInterface.Drop`
  (`PrimitiveComponent.SetSimulatePhysics` (`self.StaticMeshComponent`) true)
  (`self.K2_DetachFromActor` "KeepWorld" "KeepWorld" "KeepWorld"))

(event `Circuit Open`
  (set `self.EQ Resist` 0.0)
  (set `self.CircuitClosed` false)
  (set `self.Current` 0.0))

(event `/Game/Blueprint/PassCurrent.Pass Current`
  (params (Current :type "Float (single-precision)") (Resistance :type "Float (single-precision)") (`Closed Circuit` :type Boolean) (Passer :type "Object Object Reference") (`Nodal Current` :type "Float (single-precision)") (`Nodal Resistance` :type "Float (single-precision)") (`Node Mode` :type "/Game/Blueprint/NodeEnum Enum" :default "NewEnumerator0"))
  (set `self.EQ Resist` Resistance)
  (set `self.CircuitClosed` true)
  (set `self.Current` (/ (`KismetMathLibrary.Conv_IntToDouble` (`self.Voltage`)) (`self.EQ Resist`)))
  (`KismetSystemLibrary.RetriggerableDelay` 0.1)
  (`self.Circuit Open`))

(event `self.ReceiveTick`
  (params (DeltaSeconds :type "Float (single-precision)"))
  (if (`KismetSystemLibrary.IsValid` (`self.Postive Cable Cap`))
    (if (`self.CircuitClosed`)
      (message `/Game/Blueprint/PassCurrent.Pass Current` (`self.Postive Cable Cap`) (`self.Current`) 0.0 true null 0.0 0.0 "NewEnumerator0")
      (else
        (message `/Game/Blueprint/PassCurrent.Pass Current` (`self.Postive Cable Cap`) 0.0 0.0 false null 0.0 0.0 "NewEnumerator0")
        (message `/Game/Blueprint/PassCurrent.Pass Current` (`self.Neg Cable Cap`) 0.0 0.0 false null 0.0 0.0 "NewEnumerator0")))))

(event `self.Pos Term Collision.OnComponentBeginOverlap`
  (params (OverlappedComponent :type "PrimitiveComponent Object Reference") (OtherActor :type "Actor Object Reference") (OtherComp :type "PrimitiveComponent Object Reference") (OtherBodyIndex :type Integer) (bFromSweep :type Boolean) (SweepResult :type "HitResult Structure (by ref)"))
  (bind _pos_term_collision (`self.Pos Term Collision`))
  ;[1 1 1] Connect
  (bind _ascable_caps (cast `/Game/Blueprint/CircuitElements/CableCaps` OtherActor))
  (if (and (!= _ascable_caps (`self.Neg Cable Cap`)) (!= _ascable_caps (`self.Postive Cable Cap`)))
    (if (`/Game/Blueprint/CircuitElements/CableCaps.Coupled?` _ascable_caps)
      _
      (elif (not (`self.Pos Term Con?`))
        (set `self.Pos Term Con?` true)
        (`/Game/Blueprint/CircuitElements/CableCaps.Connect to` _ascable_caps (`SceneComponent.K2_GetComponentRotation` _pos_term_collision) (`SceneComponent.K2_GetComponentLocation` _pos_term_collision) self)
        (set `self.Postive Cable Cap` _ascable_caps)))))

(event `self.Pos Term Collision.OnComponentEndOverlap`
  (params (OverlappedComponent :type "PrimitiveComponent Object Reference") (OtherActor :type "Actor Object Reference") (OtherComp :type "PrimitiveComponent Object Reference") (OtherBodyIndex :type Integer))
  ;[1 1 1] Disconnect
  (bind _ascable_caps (cast `/Game/Blueprint/CircuitElements/CableCaps` OtherActor))
  (if (== OtherActor (`self.Postive Cable Cap`))
    (set `/Game/Blueprint/CircuitElements/CableCaps.Coupled?` false _ascable_caps)
    (set `self.Pos Term Con?` false)
    (set `/Game/Blueprint/CircuitElements/CableCaps.Owning Actor` null (`self.Postive Cable Cap`))
    (`self.Circuit Open`)
    (set `self.Postive Cable Cap` null)
    (`GameplayStatics.PlaySoundAtLocation` "/Game/Audio/cartoonpop.cartoonpop" (`self.K2_GetActorLocation`))
    (`KismetSystemLibrary.PrintString` "DROPPED")))

(event `self.Neg Term Collision.OnComponentBeginOverlap`
  (params (OverlappedComponent :type "PrimitiveComponent Object Reference") (OtherActor :type "Actor Object Reference") (OtherComp :type "PrimitiveComponent Object Reference") (OtherBodyIndex :type Integer) (bFromSweep :type Boolean) (SweepResult :type "HitResult Structure (by ref)"))
  (bind _neg_term_collision (`self.Neg Term Collision`))
  ;[1 1 1] Connect
  (bind _ascable_caps (cast `/Game/Blueprint/CircuitElements/CableCaps` OtherActor))
  (if (and (!= _ascable_caps (`self.Postive Cable Cap`)) (!= _ascable_caps (`self.Neg Cable Cap`)))
    (if (`/Game/Blueprint/CircuitElements/CableCaps.Coupled?` _ascable_caps)
      _
      (elif (not (`self.Neg Term Con?`))
        (set `self.Neg Term Con?` true)
        (`/Game/Blueprint/CircuitElements/CableCaps.Connect to` _ascable_caps (`SceneComponent.K2_GetComponentRotation` _neg_term_collision) (`SceneComponent.K2_GetComponentLocation` _neg_term_collision) self)
        (set `self.Neg Cable Cap` _ascable_caps)))))

(event `self.Neg Term Collision.OnComponentEndOverlap`
  (params (OverlappedComponent :type "PrimitiveComponent Object Reference") (OtherActor :type "Actor Object Reference") (OtherComp :type "PrimitiveComponent Object Reference") (OtherBodyIndex :type Integer))
  ;[1 1 1] Disconnect
  (bind _ascable_caps (cast `/Game/Blueprint/CircuitElements/CableCaps` OtherActor))
  (if (== OtherActor (`self.Neg Cable Cap`))
    (set `/Game/Blueprint/CircuitElements/CableCaps.Coupled?` false _ascable_caps)
    (set `self.Neg Term Con?` false)
    (set `/Game/Blueprint/CircuitElements/CableCaps.Owning Actor` null (`self.Neg Cable Cap`))
    (`self.Circuit Open`)
    (set `self.Neg Cable Cap` null)
    (`GameplayStatics.PlaySoundAtLocation` "/Game/Audio/cartoonpop.cartoonpop" (`self.K2_GetActorLocation`))
    (`KismetSystemLibrary.PrintString` "DROPPED")))

(event `self.UpButCol.OnComponentBeginOverlap`
  (params (OverlappedComponent :type "PrimitiveComponent Object Reference") (OtherActor :type "Actor Object Reference") (OtherComp :type "PrimitiveComponent Object Reference") (OtherBodyIndex :type Integer) (bFromSweep :type Boolean) (SweepResult :type "HitResult Structure (by ref)"))
  ;[1 1 1] Up Button
  (cast `/Game/Blueprint/BP_MotionController` OtherActor)
  (if (< (`self.Voltage`) (`self.Voltage upper limit`))
    (`/Engine/EditorBlueprintResources/StandardMacros.IncrementInt` (`self.Voltage`))))

(event `self.UpButCol.OnComponentEndOverlap`
  (params (OverlappedComponent :type "PrimitiveComponent Object Reference") (OtherActor :type "Actor Object Reference") (OtherComp :type "PrimitiveComponent Object Reference") (OtherBodyIndex :type Integer))
  (`PrimitiveComponent.SetMaterial` (`self.UPBUT`) 0 "/Game/StarterContent/Materials/M_Basic_Wall.M_Basic_Wall"))

(event `self.DownButCol.OnComponentBeginOverlap`
  (params (OverlappedComponent :type "PrimitiveComponent Object Reference") (OtherActor :type "Actor Object Reference") (OtherComp :type "PrimitiveComponent Object Reference") (OtherBodyIndex :type Integer) (bFromSweep :type Boolean) (SweepResult :type "HitResult Structure (by ref)"))
  ;[1 1 1] Down Button
  (cast `/Game/Blueprint/BP_MotionController` OtherActor)
  (if (> (`self.Voltage`) (`self.Voltage lower limit`))
    (`/Engine/EditorBlueprintResources/StandardMacros.DecrementInt` (`self.Voltage`))))

(event `self.DownButCol.OnComponentEndOverlap`
  (params (OverlappedComponent :type "PrimitiveComponent Object Reference") (OtherActor :type "Actor Object Reference") (OtherComp :type "PrimitiveComponent Object Reference") (OtherBodyIndex :type Integer))
  (`PrimitiveComponent.SetMaterial` (`self.DownBut`) 0 "/Game/StarterContent/Materials/M_Basic_Wall.M_Basic_Wall"))

(fn `UserConstructionScript`)