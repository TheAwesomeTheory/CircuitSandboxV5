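; Cable end cap for a circuit-building game, which motion controllers can pick up and drop and which snaps onto circuit elements.
; ConnectTo, guarded by a Coupled flag, disables physics, attaches the cap to the element, stores it as OwningActor and plays a snap sound.
; Current, resistance and nodal data entering one cap pass to its PartnerCap, which forwards them to its own OwningActor.
; Pickup clears OwningActor but leaves Coupled set, and the disconnect message is unwired.
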(event `Pass Current Second Cap`
  (params (Current :type "Float (double-precision)") (`Resistance In` :type "Float (double-precision)") (`Closed Circuit` :type Boolean) (Passer :type "Object Object Reference") (`Nodal Current` :type "Float (double-precision)") (`Nodal Resistance` :type "Float (double-precision)") (`Node Mode` :type "/Game/Blueprint/NodeEnum Enum"))
  (message `/Game/Blueprint/PassCurrent.Pass Current` (`self.Owning Actor`) Current `Resistance In` `Closed Circuit` self `Nodal Current` `Nodal Resistance` `Node Mode`))

(event `/Game/Blueprint/PassCurrent.Pass Current`
  (params (Current :type "Float (single-precision)") (Resistance :type "Float (single-precision)") (`Closed Circuit` :type Boolean) (Passer :type "Object Object Reference") (`Nodal Current` :type "Float (single-precision)") (`Nodal Resistance` :type "Float (single-precision)") (`Node Mode` :type "/Game/Blueprint/NodeEnum Enum" :default "NewEnumerator0"))
  (`self.Pass Current Second Cap` (`self.PartnerCap`) Current Resistance `Closed Circuit` self `Nodal Current` `Nodal Resistance` `Node Mode`))

(event `/Game/Blueprint/PickupActorInterface.Pickup`
  (params (AttachTo :type "SceneComponent Object Reference") (GrabbedComponent :type "SceneComponent Object Reference"))
  (`PrimitiveComponent.SetSimulatePhysics` (`self.StaticMeshComponent`) false)
  (`SceneComponent.K2_AttachToComponent` (`self.K2_GetRootComponent`) AttachTo "None" "KeepWorld" "KeepWorld" "KeepWorld" false)
  (set `self.Owning Actor` null))

(event `/Game/Blueprint/PickupActorInterface.Drop`
  (params (`Drop er` :type "SceneComponent Object Reference"))
  (`PrimitiveComponent.SetSimulatePhysics` (`self.StaticMeshComponent`) true)
  (`self.K2_DetachFromActor` "KeepWorld" "KeepWorld" "KeepWorld"))

(fn `Connect to`
  (params (`Connect Rotation` :type "Rotator Structure") (`Connect Location` :type "Vector Structure") (`Parent Actor` :type "Actor Object Reference"))
  (if (not (`self.Coupled?`))
    (set `self.Coupled?` true)
    (`PrimitiveComponent.SetSimulatePhysics` (`self.StaticMeshComponent`) false)
    (`self.K2_SetActorLocation` `Connect Location`)
    (`self.K2_SetActorRotation` `Connect Rotation`)
    (`self.K2_DetachFromActor` "KeepWorld" "KeepWorld" "KeepWorld")
    (`self.K2_AttachToActor` `Parent Actor` "None" "KeepWorld" "KeepWorld" "KeepWorld")
    (set `self.Owning Actor` `Parent Actor`)
    (`GameplayStatics.PlaySoundAtLocation` "/Game/Audio/snap_togther.snap_togther" (`self.K2_GetActorLocation`))))

(fn `UserConstructionScript`)