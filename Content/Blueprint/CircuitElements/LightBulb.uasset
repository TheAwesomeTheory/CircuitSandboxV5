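; A light bulb circuit component that can be picked up by a motion controller and glows with the current passing through it.
; Cable caps couple to its two terminals on overlap, and PassCurrent relays current to the opposite cap with added resistance.
; A retriggerable delay zeroes the stored current when pulses stop.
; Tick drives material brightness from current; exceeding the threshold triggers a one-time brightness timeline, then destructible damage, particles and sound.
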(event `/Game/Blueprint/PassCurrent.Pass Current`
  (params (Current :type "Float (single-precision)") (Resistance :type "Float (single-precision)") (`Closed Circuit` :type Boolean) (Passer :type "Object Object Reference") (`Nodal Current` :type "Float (single-precision)") (`Nodal Resistance` :type "Float (single-precision)") (`Node Mode` :type "/Game/Blueprint/NodeEnum Enum" :default "NewEnumerator0"))
  (bind _returnvalue (+ (`self.resistance`) Resistance))
  (`|ExecutionSequence`
    (:`then_0`
      (`KismetSystemLibrary.RetriggerableDelay` 0.1)
      (set `self.Current` 0.0))
    (:`then_1`
      (if (== Passer (`self.cap 1`))
        (message `/Game/Blueprint/PassCurrent.Pass Current` (`self.cap 2`) Current _returnvalue `Closed Circuit` null `Nodal Current` `Nodal Resistance` `Node Mode`)
        (else
          (message `/Game/Blueprint/PassCurrent.Pass Current` (`self.cap 1`) Current _returnvalue `Closed Circuit` null `Nodal Current` `Nodal Resistance` `Node Mode`))))
    (:`then_2`
      (set `self.Current` Current))))

(event `self.ReceiveTick`
  (params (DeltaSeconds :type "Float (single-precision)"))
  (if (not (`self.Exploded?`))
    (`MeshComponent.SetScalarParameterValueOnMaterials` (`self.StaticMesh`) "Birghtness" (`self.Current`))
    (if (> (`self.Current`) (`self.Thresh Hold`))
      (`/Engine/EditorBlueprintResources/StandardMacros.DoOnce` false
        (:`Completed`
          (set `self.Exploded?` true)
          (bind (_direction _brightness) (`Timeline|Timeline_0`)
            (:`Update`
              (`MeshComponent.SetScalarParameterValueOnMaterials` (`self.StaticMesh`) "Birghtness" _brightness))
            (:`Finished`
              (`DestructibleComponent.ApplyDamage` (`self.Destructible`) 100.0 (`SceneComponent.K2_GetComponentLocation` (`self.Destructible`)) (`KismetMathLibrary.MakeVector` 0.0 0.0 1.0) 100.0)
              (`ActorComponent.Activate` (`self.ParticleSystem`) false)
              (`MeshComponent.SetScalarParameterValueOnMaterials` (`self.StaticMesh`) "Birghtness" 0.0)
              (`GameplayStatics.PlaySoundAtLocation` "/Game/Audio/LightbulbExplode_ShorterLouder.LightbulbExplode_ShorterLouder" (`self.K2_GetActorLocation`) (struct) 0.7))))))))

(event `/Game/Blueprint/PickupActorInterface.Pickup`
  (params (AttachTo :type "SceneComponent Object Reference") (GrabbedComponent :type "SceneComponent Object Reference"))
  ;[1 1 1] Interaction Blueprints
  (`PrimitiveComponent.SetSimulatePhysics` (`self.StaticMeshComponent`) false)
  (`SceneComponent.K2_AttachToComponent` (`self.K2_GetRootComponent`) AttachTo "None" "KeepWorld" "KeepWorld" "KeepWorld" false))

(event `/Game/Blueprint/PickupActorInterface.Drop`
  ;[1 1 1] Interaction Blueprints
  (`PrimitiveComponent.SetSimulatePhysics` (`self.StaticMeshComponent`) true)
  (`self.K2_DetachFromActor` "KeepWorld" "KeepWorld" "KeepWorld"))

(event `self.Sphere1.OnComponentBeginOverlap`
  (params (OverlappedComponent :type "PrimitiveComponent Object Reference") (OtherActor :type "Actor Object Reference") (OtherComp :type "PrimitiveComponent Object Reference") (OtherBodyIndex :type Integer) (bFromSweep :type Boolean) (SweepResult :type "HitResult Structure (by ref)"))
  (bind _sphere1 (`self.Sphere1`))
  ;[1 1 1] Connect
  (bind _ascable_caps (cast `/Game/Blueprint/CircuitElements/CableCaps` OtherActor))
  (if (!= _ascable_caps (`self.cap 1`))
    (if (`/Game/Blueprint/CircuitElements/CableCaps.Coupled?` _ascable_caps)
      _
      (elif (not (`self.connection 2`))
        (set `self.connection 2` true)
        (`/Game/Blueprint/CircuitElements/CableCaps.Connect to` _ascable_caps (`SceneComponent.K2_GetComponentRotation` _sphere1) (`SceneComponent.K2_GetComponentLocation` _sphere1) self)
        (set `self.cap 2` _ascable_caps)))))

(event `self.Cap 1 collision.OnComponentBeginOverlap`
  (params (OverlappedComponent :type "PrimitiveComponent Object Reference") (OtherActor :type "Actor Object Reference") (OtherComp :type "PrimitiveComponent Object Reference") (OtherBodyIndex :type Integer) (bFromSweep :type Boolean) (SweepResult :type "HitResult Structure (by ref)"))
  (bind _cap_1_collision (`self.Cap 1 collision`))
  ;[1 1 1] Connect
  (bind _ascable_caps (cast `/Game/Blueprint/CircuitElements/CableCaps` OtherActor))
  (if (and (!= _ascable_caps (`self.cap 2`)) (!= _ascable_caps (`self.cap 1`)))
    (if (`/Game/Blueprint/CircuitElements/CableCaps.Coupled?` _ascable_caps)
      _
      (elif (not (`self.connection 1`))
        (set `self.connection 1` true)
        (`/Game/Blueprint/CircuitElements/CableCaps.Connect to` _ascable_caps (`SceneComponent.K2_GetComponentRotation` _cap_1_collision) (`SceneComponent.K2_GetComponentLocation` _cap_1_collision) self)
        (set `self.cap 1` _ascable_caps)))))

(event `self.Cap 1 collision.OnComponentEndOverlap`
  (params (OverlappedComponent :type "PrimitiveComponent Object Reference") (OtherActor :type "Actor Object Reference") (OtherComp :type "PrimitiveComponent Object Reference") (OtherBodyIndex :type Integer))
  (bind _ascable_caps (cast `/Game/Blueprint/CircuitElements/CableCaps` OtherActor))
  (if (== OtherActor (`self.cap 1`))
    (set `/Game/Blueprint/CircuitElements/CableCaps.Coupled?` false _ascable_caps)
    (set `self.connection 1` false)
    (set `/Game/Blueprint/CircuitElements/CableCaps.Owning Actor` null (`self.cap 1`))
    (set `self.cap 1` null)
    (`GameplayStatics.PlaySoundAtLocation` "/Game/Audio/cartoonpop.cartoonpop" (`self.K2_GetActorLocation`))))

(event `self.Sphere1.OnComponentEndOverlap`
  (params (OverlappedComponent :type "PrimitiveComponent Object Reference") (OtherActor :type "Actor Object Reference") (OtherComp :type "PrimitiveComponent Object Reference") (OtherBodyIndex :type Integer))
  (bind _ascable_caps (cast `/Game/Blueprint/CircuitElements/CableCaps` OtherActor))
  (if (== OtherActor (`self.cap 2`))
    (set `/Game/Blueprint/CircuitElements/CableCaps.Coupled?` false _ascable_caps)
    (set `self.connection 2` false)
    (set `/Game/Blueprint/CircuitElements/CableCaps.Owning Actor` null (`self.cap 2`))
    (set `self.cap 2` null)
    (`GameplayStatics.PlaySoundAtLocation` "/Game/Audio/cartoonpop.cartoonpop" (`self.K2_GetActorLocation`))))

(fn `UserConstructionScript`)