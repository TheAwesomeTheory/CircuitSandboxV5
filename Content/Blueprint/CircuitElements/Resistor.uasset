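; VR circuit resistor that players grab with motion controllers and wire between two cable ends.
; Each end sphere couples an uncoupled CableCaps on overlap and releases it with a pop sound on end overlap.
; PassCurrent forwards the signal out the opposite cap with its resistance added, storing the current until a retriggerable delay zeroes it when pulses stop.
; Pickup creates a physics handle that follows the controller each tick.
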(event `/Game/Blueprint/PassCurrent.Pass Current`
  (params (Current :type "Float (single-precision)") (Resistance :type "Float (single-precision)") (`Closed Circuit` :type Boolean) (Passer :type "Object Object Reference") (`Nodal Current` :type "Float (single-precision)") (`Nodal Resistance` :type "Float (single-precision)") (`Node Mode` :type "/Game/Blueprint/NodeEnum Enum" :default "NewEnumerator0") (`VOLTAGE SOURCE` :type "Object Object Reference"))
  (bind _returnvalue (+ Resistance (`self.Reistance`)))
  (`|ExecutionSequence`
    (:`then_0`
      (`KismetSystemLibrary.RetriggerableDelay` 0.1)
      (set `self.Current` 0.0))
    (:`then_1`
      (if (== Passer (`self.NewVar_0`))
        (message `/Game/Blueprint/PassCurrent.Pass Current` (`self.NewVar_1`) Current _returnvalue `Closed Circuit` null `Nodal Current` `Nodal Resistance` `Node Mode` `VOLTAGE SOURCE`)
        (else
          (message `/Game/Blueprint/PassCurrent.Pass Current` (`self.NewVar_0`) Current _returnvalue `Closed Circuit` null `Nodal Current` `Nodal Resistance` `Node Mode` `VOLTAGE SOURCE`))))
    (:`then_2`
      (set `self.Current` Current))))

(event `/Game/Blueprint/PickupActorInterface.Pickup`
  (params (AttachTo :type "SceneComponent Object Reference") (GrabbedComponent :type "SceneComponent Object Reference"))
  (bind _motion_controller (`self.Motion Controller`))
  (bind _output_get (set `self.Motion Controller` AttachTo))
  (`self.ClearPreviousHolder`)
  (`self.K2_SetActorLocation` (+ (* (`SceneComponent.GetForwardVector` _output_get) (`self.Hold distance`)) (`SceneComponent.K2_GetComponentLocation` _output_get)))
  (bind _returnvalue (`AddComponent|NODE_AddPhysicsHandleComponent-0`))
  (bind _output_get_2 (set `self.physics handle` _returnvalue))
  (`PhysicsHandleComponent.GrabComponentAtLocationWithRotation` _output_get_2 (`self.StaticMeshComponent`) "None" (`SceneComponent.K2_GetComponentLocation` _motion_controller) (`SceneComponent.K2_GetComponentRotation` _motion_controller)))

(event `ClearPreviousHolder`
  (bind _physics_handle (`self.physics handle`))
  (`PhysicsHandleComponent.ReleaseComponent` _physics_handle :!label _label)
  (`ActorComponent.K2_DestroyComponent` _physics_handle))

(event `/Game/Blueprint/PickupActorInterface.Drop`
  (params (`Drop er` :type "SceneComponent Object Reference"))
  (if (== `Drop er` (`self.Motion Controller`))
    (goto _label)))

(event `self.ReceiveTick`
  (params (DeltaSeconds :type "Float (single-precision)"))
  (bind _motion_controller (`self.Motion Controller`))
  (`/Engine/EditorBlueprintResources/StandardMacros.IsValid` _motion_controller
    (:`Is Valid`
      (`PhysicsHandleComponent.SetTargetLocationAndRotation` (`self.physics handle`) (`SceneComponent.K2_GetComponentLocation` _motion_controller) (`SceneComponent.K2_GetComponentRotation` _motion_controller)))))

(event `self.Sphere1.OnComponentBeginOverlap`
  (params (OverlappedComponent :type "PrimitiveComponent Object Reference") (OtherActor :type "Actor Object Reference") (OtherComp :type "PrimitiveComponent Object Reference") (OtherBodyIndex :type Integer) (bFromSweep :type Boolean) (SweepResult :type "HitResult Structure (by ref)"))
  (bind _sphere1 (`self.Sphere1`))
  ;[1 1 1] connect
  (bind _ascable_caps (cast `/Game/Blueprint/CircuitElements/CableCaps` OtherActor))
  (if (and (!= (`self.NewVar_1`) _ascable_caps) (!= _ascable_caps (`self.NewVar_0`)))
    (if (`/Game/Blueprint/CircuitElements/CableCaps.Coupled?` _ascable_caps)
      _
      (elif (not (`self.CON 2`))
        (set `self.CON 2` true)
        (`/Game/Blueprint/CircuitElements/CableCaps.Connect to` _ascable_caps (`SceneComponent.K2_GetComponentRotation` _sphere1) (`SceneComponent.K2_GetComponentLocation` _sphere1) self)
        (set `self.NewVar_1` _ascable_caps)))))

(event `self.Sphere.OnComponentBeginOverlap`
  (params (OverlappedComponent :type "PrimitiveComponent Object Reference") (OtherActor :type "Actor Object Reference") (OtherComp :type "PrimitiveComponent Object Reference") (OtherBodyIndex :type Integer) (bFromSweep :type Boolean) (SweepResult :type "HitResult Structure (by ref)"))
  (bind _sphere (`self.Sphere`))
  ;[1 1 1] connect
  (bind _ascable_caps (cast `/Game/Blueprint/CircuitElements/CableCaps` OtherActor))
  (if (and (!= _ascable_caps (`self.NewVar_1`)) (!= _ascable_caps (`self.NewVar_0`)))
    (if (`/Game/Blueprint/CircuitElements/CableCaps.Coupled?` _ascable_caps)
      _
      (elif (not (`self.CON 1`))
        (set `self.CON 1` true)
        (`/Game/Blueprint/CircuitElements/CableCaps.Connect to` _ascable_caps (`SceneComponent.K2_GetComponentRotation` _sphere) (`SceneComponent.K2_GetComponentLocation` _sphere) self)
        (set `self.NewVar_0` _ascable_caps)))))

(event `self.Sphere.OnComponentEndOverlap`
  (params (OverlappedComponent :type "PrimitiveComponent Object Reference") (OtherActor :type "Actor Object Reference") (OtherComp :type "PrimitiveComponent Object Reference") (OtherBodyIndex :type Integer))
  ;[1 1 1] Disconnect
  (bind _ascable_caps (cast `/Game/Blueprint/CircuitElements/CableCaps` OtherActor))
  (if (== OtherActor (`self.NewVar_0`))
    (set `/Game/Blueprint/CircuitElements/CableCaps.Coupled?` false _ascable_caps)
    (set `self.CON 1` false)
    (set `/Game/Blueprint/CircuitElements/CableCaps.Owning Actor` null (`self.NewVar_0`))
    (set `self.NewVar_0` null)
    (`GameplayStatics.PlaySoundAtLocation` "/Game/Audio/cartoonpop.cartoonpop" (`self.K2_GetActorLocation`))))

(event `self.Sphere1.OnComponentEndOverlap`
  (params (OverlappedComponent :type "PrimitiveComponent Object Reference") (OtherActor :type "Actor Object Reference") (OtherComp :type "PrimitiveComponent Object Reference") (OtherBodyIndex :type Integer))
  ;[1 1 1] Disconnect
  (bind _ascable_caps (cast `/Game/Blueprint/CircuitElements/CableCaps` OtherActor))
  (if (== OtherActor (`self.NewVar_1`))
    (set `/Game/Blueprint/CircuitElements/CableCaps.Coupled?` false _ascable_caps)
    (set `self.CON 2` false)
    (set `/Game/Blueprint/CircuitElements/CableCaps.Owning Actor` null (`self.NewVar_1`))
    (set `self.NewVar_1` null)
    (`GameplayStatics.PlaySoundAtLocation` "/Game/Audio/cartoonpop.cartoonpop" (`self.K2_GetActorLocation`))))

(fn `UserConstructionScript`)