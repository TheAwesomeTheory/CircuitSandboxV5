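; Fork is a circuit junction that can be picked up and dropped, splitting one cable into two branches.
; Its three overlap sockets each couple one CableCaps and pop on disconnect.
; PassCurrent uses a node mode to forward input to both branches, then divide returning nodal current by branch resistance ratio and report parallel resistance to the first cap.
; Retriggerable delays zero branch resistances when updates stop.
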(event `self.single.OnComponentBeginOverlap`
  (params (OverlappedComponent :type "PrimitiveComponent Object Reference") (OtherActor :type "Actor Object Reference") (OtherComp :type "PrimitiveComponent Object Reference") (OtherBodyIndex :type Integer) (bFromSweep :type Boolean) (SweepResult :type "HitResult Structure (by ref)"))
  (bind _single (`self.single`))
  ;[1 1 1] connect to calbes caps
  (bind _ascable_caps (cast `/Game/Blueprint/CircuitElements/CableCaps` OtherActor))
  (if (and (!= _ascable_caps (`self.cap 2`)) (!= _ascable_caps (`self.cap 1`)) (!= _ascable_caps (`self.cap 3`)))
    (if (`/Game/Blueprint/CircuitElements/CableCaps.Coupled?` _ascable_caps)
      _
      (elif (not (`self.connection 1`))
        (set `self.connection 1` true)
        (`/Game/Blueprint/CircuitElements/CableCaps.Connect to` _ascable_caps (`SceneComponent.K2_GetComponentRotation` _single) (`SceneComponent.K2_GetComponentLocation` _single) self)
        (set `self.cap 1` _ascable_caps)))))

(event `self.single.OnComponentEndOverlap`
  (params (OverlappedComponent :type "PrimitiveComponent Object Reference") (OtherActor :type "Actor Object Reference") (OtherComp :type "PrimitiveComponent Object Reference") (OtherBodyIndex :type Integer))
  ;[1 1 1] Disconnect from cable caps
  (bind _ascable_caps (cast `/Game/Blueprint/CircuitElements/CableCaps` OtherActor))
  (if (== OtherActor (`self.cap 1`))
    (set `/Game/Blueprint/CircuitElements/CableCaps.Coupled?` false _ascable_caps)
    (set `self.connection 1` false)
    (set `/Game/Blueprint/CircuitElements/CableCaps.Owning Actor` null (`self.cap 1`))
    (set `self.cap 1` null)
    (`GameplayStatics.PlaySoundAtLocation` "/Game/Audio/cartoonpop.cartoonpop" (`self.K2_GetActorLocation`))))

(event `self.DA.OnComponentEndOverlap`
  (params (OverlappedComponent :type "PrimitiveComponent Object Reference") (OtherActor :type "Actor Object Reference") (OtherComp :type "PrimitiveComponent Object Reference") (OtherBodyIndex :type Integer))
  ;[1 1 1] Disconnect from cable caps
  (bind _ascable_caps (cast `/Game/Blueprint/CircuitElements/CableCaps` OtherActor))
  (if (== OtherActor (`self.cap 2`))
    (set `/Game/Blueprint/CircuitElements/CableCaps.Coupled?` false _ascable_caps)
    (set `self.connection 2` false)
    (set `/Game/Blueprint/CircuitElements/CableCaps.Owning Actor` null (`self.cap 2`))
    (set `self.cap 2` null)
    (`GameplayStatics.PlaySoundAtLocation` "/Game/Audio/cartoonpop.cartoonpop" (`self.K2_GetActorLocation`))))

(event `self.DA.OnComponentBeginOverlap`
  (params (OverlappedComponent :type "PrimitiveComponent Object Reference") (OtherActor :type "Actor Object Reference") (OtherComp :type "PrimitiveComponent Object Reference") (OtherBodyIndex :type Integer) (bFromSweep :type Boolean) (SweepResult :type "HitResult Structure (by ref)"))
  (bind _da (`self.DA`))
  ;[1 1 1] connect to calbes caps
  (bind _ascable_caps (cast `/Game/Blueprint/CircuitElements/CableCaps` OtherActor))
  (if (and (!= _ascable_caps (`self.cap 2`)) (!= _ascable_caps (`self.cap 1`)) (!= _ascable_caps (`self.cap 3`)))
    (if (`/Game/Blueprint/CircuitElements/CableCaps.Coupled?` _ascable_caps)
      _
      (elif (not (`self.connection 2`))
        (set `self.connection 2` true)
        (`/Game/Blueprint/CircuitElements/CableCaps.Connect to` _ascable_caps (`SceneComponent.K2_GetComponentRotation` _da) (`SceneComponent.K2_GetComponentLocation` _da) self)
        (set `self.cap 2` _ascable_caps)))))

(event `self.DB.OnComponentEndOverlap`
  (params (OverlappedComponent :type "PrimitiveComponent Object Reference") (OtherActor :type "Actor Object Reference") (OtherComp :type "PrimitiveComponent Object Reference") (OtherBodyIndex :type Integer))
  ;[1 1 1] Disconnect from cable caps
  (bind _ascable_caps (cast `/Game/Blueprint/CircuitElements/CableCaps` OtherActor))
  (if (== OtherActor (`self.cap 3`))
    (set `/Game/Blueprint/CircuitElements/CableCaps.Coupled?` false _ascable_caps)
    (set `self.connection 3` false)
    (set `/Game/Blueprint/CircuitElements/CableCaps.Owning Actor` null (`self.cap 3`))
    (set `self.cap 3` null)
    (`GameplayStatics.PlaySoundAtLocation` "/Game/Audio/cartoonpop.cartoonpop" (`self.K2_GetActorLocation`))))

(event `self.DB.OnComponentBeginOverlap`
  (params (OverlappedComponent :type "PrimitiveComponent Object Reference") (OtherActor :type "Actor Object Reference") (OtherComp :type "PrimitiveComponent Object Reference") (OtherBodyIndex :type Integer) (bFromSweep :type Boolean) (SweepResult :type "HitResult Structure (by ref)"))
  (bind _db (`self.DB`))
  ;[1 1 1] connect to calbes caps
  (bind _ascable_caps (cast `/Game/Blueprint/CircuitElements/CableCaps` OtherActor))
  (if (and (!= _ascable_caps (`self.cap 2`)) (!= _ascable_caps (`self.cap 1`)) (!= (`self.cap 3`) _ascable_caps))
    (if (`/Game/Blueprint/CircuitElements/CableCaps.Coupled?` _ascable_caps)
      _
      (elif (not (`self.connection 3`))
        (set `self.connection 3` true)
        (`/Game/Blueprint/CircuitElements/CableCaps.Connect to` _ascable_caps (`SceneComponent.K2_GetComponentRotation` _db) (`SceneComponent.K2_GetComponentLocation` _db) self)
        (set `self.cap 3` _ascable_caps)))))

(event `/Game/Blueprint/PickupActorInterface.Pickup`
  (params (AttachTo :type "SceneComponent Object Reference") (GrabbedComponent :type "SceneComponent Object Reference"))
  ;[1 1 1] Pickup/Drop Logic
  (`PrimitiveComponent.SetSimulatePhysics` (`self.StaticMeshComponent`) false)
  (`SceneComponent.K2_AttachToComponent` (`self.K2_GetRootComponent`) AttachTo "None" "KeepWorld" "KeepWorld" "KeepWorld" false))

(event `/Game/Blueprint/PickupActorInterface.Drop`
  (params (`Drop er` :type "SceneComponent Object Reference"))
  ;[1 1 1] Pickup/Drop Logic
  (`PrimitiveComponent.SetSimulatePhysics` (`self.StaticMeshComponent`) true)
  (`self.K2_DetachFromActor` "KeepWorld" "KeepWorld" "KeepWorld"))

(event `/Game/Blueprint/PassCurrent.Pass Current`
  (params (Current :type "Float (single-precision)") (Resistance :type "Float (single-precision)") (`Closed Circuit` :type Boolean) (Passer :type "Object Object Reference") (`Nodal Current` :type "Float (single-precision)") (`Nodal Resistance` :type "Float (single-precision)") (`Node Mode` :type "/Game/Blueprint/NodeEnum Enum" :default "NewEnumerator0"))
  (bind _resistance_2 (`self.Resistance 2`))
  (bind _resistance_1 (`self.Resistance 1`))
  (bind _cap_2 (`self.cap 2`))
  (bind _cap_3 (`self.cap 3`))
  (`self.Check Nodal Mode` `Node Mode`
    (:`Clear`
      (`self.Update Incoming Values` Current Resistance `Closed Circuit` Passer `Nodal Current` `Nodal Resistance`
        (:`Done`
          (`/Game/Blueprint/CircuitElements/CableCaps.Pass Current` (`self.cap 2`) 0.0 0.0 false null (`self.Input Current`) (`self.Input Resistance`) "NewEnumerator1")
          (`/Game/Blueprint/CircuitElements/CableCaps.Pass Current` (`self.cap 3`) 0.0 0.0 false null (`self.Input Current`) (`self.Input Resistance`) "NewEnumerator1"))))
    (:`Send Current Back`
      (`self.Update Incoming Values` Current Resistance `Closed Circuit` Passer `Nodal Current` `Nodal Resistance`
        (:`Done`
          (`self.Update Resistances`
            (:`Cap 2`
              (`/Game/Blueprint/CircuitElements/CableCaps.Pass Current` _cap_2 (* (/ _resistance_1 (+ _resistance_1 (`self.Resistance 2`))) (`self.Input Nodal current`)) 0.0 false _cap_2 0.0 0.0 "NewEnumerator3"))
            (:`Cap 3`
              (`/Game/Blueprint/CircuitElements/CableCaps.Pass Current` _cap_3 (* (/ _resistance_2 (+ _resistance_2 (`self.Resistance 1`))) (`self.Input Nodal current`)) 0.0 false _cap_3 0.0 0.0 "NewEnumerator3")))
          (`/Game/Blueprint/CircuitElements/CableCaps.Pass Current` (`self.cap 1`) (`self.Input Nodal current`) (+ (`self.Input Nodal Resistance`) (/ 1.0 (+ (/ 1.0 (`self.Resistance 1`)) (/ 1.0 (`self.Resistance 2`))))) false null 0.0 0.0 "NewEnumerator0"))))))

(fn `UserConstructionScript`)