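; PDA actor for VR that can be picked up and spawns an Ohm's Law billboard when its button is pressed.
; Pickup and Drop toggle the box's physics, attach or detach the actor, and track the held state, with Pickup recording the owning hand.
; OhmsLaw spawns a BillBoard owned by the third CableCaps actor found in the level and prints a debug message.
; An unconnected held-hand check never runs.
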(event `/Game/Blueprint/ButtonInterface.Button Pressed`
  (params (`Button Index` :type Integer))
  (`self.Ohm's Law`))

(event `/Game/Blueprint/PickupActorInterface.Pickup`
  (params (AttachTo :type "SceneComponent Object Reference") (GrabbedComponent :type "SceneComponent Object Reference"))
  ;[1 1 1] Interaction Blueprints
  (`PrimitiveComponent.SetSimulatePhysics` (`self.Box`) false)
  (bind _asmotion_controller_component (cast `MotionControllerComponent` AttachTo))
  (set `self.Owning Hand` _asmotion_controller_component)
  (`SceneComponent.K2_AttachToComponent` (`self.K2_GetRootComponent`) AttachTo "None" "KeepWorld" "KeepWorld" "KeepWorld" false)
  (set `self.Held?` true))

(event `/Game/Blueprint/PickupActorInterface.Drop`
  ;[1 1 1] Interaction Blueprints
  (`PrimitiveComponent.SetSimulatePhysics` (`self.Box`) true)
  (`self.K2_DetachFromActor` "KeepWorld" "KeepWorld" "KeepWorld")
  (set `self.Held?` false))

(fn `Ohm's Law`
  (locals (NewLocalVar_0 :type "Array of /Game/LowPolyText/DataStructs/TextData Structure") (`Owning Actor` :type "Actor Object Reference" :default null))
  (bind _outactors (`GameplayStatics.GetAllActorsOfClass` "/Game/Blueprint/CircuitElements/CableCaps.CableCaps_C"))
  (`|SpawnActorFromClass` "/Game/Blueprint/BillBoard.BillBoard_C" (`KismetMathLibrary.MakeTransform` (0.0 0.0 600.0)) "Undefined" "OverrideRootScale" null 35.0 15.0 (`KismetArrayLibrary.Array_Get` _outactors 2) 10.0 (`local.NewLocalVar_0`))
  (`KismetSystemLibrary.PrintString` "Tried To Spawn Billboard"))

(fn `UserConstructionScript`)