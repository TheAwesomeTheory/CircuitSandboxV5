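; Alarm light actor that flashes a rotating spotlight and sounds a fire alarm when an emergency is triggered.
; Tick continuously spins the SpotLight around its yaw axis.
; EmergencyHasHappened swaps the mesh's light material, raises spotlight intensity and plays the quiet alarm sound three times using delays, then restores the off state.
; An On flag blocks retriggering while the sequence runs.
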(event `self.ReceiveTick`
  (params (DeltaSeconds :type "Float (single-precision)"))
  (`SceneComponent.K2_AddLocalRotation` (`self.SpotLight`) (`KismetMathLibrary.MakeRotator` 0.0 0.0 (* DeltaSeconds 180.0)) false false))

(event `/Game/Blueprint/Emergency.Emergency has happened`
  (params (NewParam :type Boolean))
  (if (not (`self.on?`))
    (set `self.on?` true)
    (`PrimitiveComponent.SetMaterial` (`self.StaticMeshComponent`) 1 "/Game/Materials/Light_4.Light_4")
    (`LightComponent.SetIntensity` (`self.SpotLight`) 15000.0)
    (`GameplayStatics.SpawnSoundAtLocation` "/Game/Audio/FireAlarm.FireAlarm" (`self.K2_GetActorLocation`) (struct) 0.01)
    (`KismetSystemLibrary.Delay` 2.89)
    (`GameplayStatics.SpawnSoundAtLocation` "/Game/Audio/FireAlarm.FireAlarm" (`self.K2_GetActorLocation`) (struct) 0.01)
    (`KismetSystemLibrary.Delay` 2.89)
    (`GameplayStatics.SpawnSoundAtLocation` "/Game/Audio/FireAlarm.FireAlarm" (`self.K2_GetActorLocation`) (struct) 0.01)
    (`KismetSystemLibrary.Delay` 1.0)
    (`LightComponent.SetIntensity` (`self.SpotLight`) 0.0)
    (`PrimitiveComponent.SetMaterial` (`self.StaticMeshComponent`) 1 "/Game/Materials/M_PDA_1.M_PDA_1")
    (set `self.on?` false)))

(fn `UserConstructionScript`)