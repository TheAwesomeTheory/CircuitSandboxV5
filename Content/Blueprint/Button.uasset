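; A physical VR button that a motion controller fingertip pushes to send its index to the owning actor.
; Physics runs only while the fingertip overlaps the Box; otherwise Tick holds the button at rest above its Plane.
; Per-axis spring-like forces constrain it, snapping back sideways drift and dropping collision when pushed too deep.
; Passing the trigger depth fires once, toggling the material, and re-arms near the rest point.
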(event `self.ReceiveBeginPlay`
  (`PrimitiveComponent.SetSimulatePhysics` (`self.Button`) false))

(event `self.ReceiveTick`
  (params (DeltaSeconds :type "Float (single-precision)"))
  (bind _returnvalue (`SceneComponent.GetUpVector` (`self.Plane`)))
  (bind _returnvalue_2 (`KismetMathLibrary.ProjectVectorOnToVector` (- (`SceneComponent.K2_GetComponentLocation` (`self.Button`)) (`SceneComponent.K2_GetComponentLocation` (`self.Plane`))) (`SceneComponent.GetRightVector` (`self.Plane`))))
  (bind _returnvalue_3 (`KismetMathLibrary.ProjectVectorOnToVector` (- (`SceneComponent.K2_GetComponentLocation` (`self.Button`)) (`SceneComponent.K2_GetComponentLocation` (`self.Plane`))) (`SceneComponent.GetForwardVector` (`self.Plane`))))
  (bind _returnvalue_4 (+ (`SceneComponent.K2_GetComponentLocation` (`self.Plane`)) (* _returnvalue (`self.Button Height`))))
  (bind _returnvalue_5 (`KismetMathLibrary.ProjectVectorOnToVector` (- (`SceneComponent.K2_GetComponentLocation` (`self.Button`)) _returnvalue_4) _returnvalue))
  (bind _returnvalue_6 (`KismetMathLibrary.VSize` _returnvalue_5))
  (`|ExecutionSequence`
    (:`then_0`
      (if (`self.Hand Overlapping?`)
        (`KismetSystemLibrary.PrintString` "Physicsing")
        (`|ExecutionSequence`
          (:`then_0`
            (if (> (`KismetMathLibrary.VSize` _returnvalue_2) 15.0)
              (`PrimitiveComponent.SetCollisionEnabled` (`self.Button`) "NoCollision")
              (`PrimitiveComponent.SetAllPhysicsLinearVelocity` (`self.Button`) (0.0 0.0 0.0) false)
              (`SceneComponent.K2_SetWorldLocation` (`self.Button`) _returnvalue_4 false false)
              (`SceneComponent.K2_SetWorldRotation` (`self.Button`) (`SceneComponent.K2_GetComponentRotation` (`self.Plane`)) false false)
              (`PrimitiveComponent.SetCollisionEnabled` (`self.Button`) "QueryAndPhysics")
              (else
                (`PrimitiveComponent.AddForce` (`self.Button`) (* _returnvalue_2 (`self.button Force Multiplier x/y`)) "None" true))))
          (:`then_1`
            (if (> (`KismetMathLibrary.VSize` _returnvalue_3) 15.0)
              (`PrimitiveComponent.SetCollisionEnabled` (`self.Button`) "NoCollision")
              (`PrimitiveComponent.SetAllPhysicsLinearVelocity` (`self.Button`) (0.0 0.0 0.0) false)
              (`SceneComponent.K2_SetWorldLocation` (`self.Button`) _returnvalue_4 false false)
              (`SceneComponent.K2_SetWorldRotation` (`self.Button`) (`SceneComponent.K2_GetComponentRotation` (`self.Plane`)) false false)
              (`PrimitiveComponent.SetCollisionEnabled` (`self.Button`) "QueryAndPhysics")
              (else
                (`PrimitiveComponent.AddForce` (`self.Button`) (* _returnvalue_3 (`self.button Force Multiplier x/y`)) "None" true))))
          (:`then_3`
            (if (> _returnvalue_6 (`self.Button Reset Depth`))
              (`PrimitiveComponent.SetCollisionEnabled` (`self.Button`) "NoCollision")
              (else
                (`PrimitiveComponent.AddForce` (`self.Button`) (* _returnvalue_5 (`self.Button force Multiplier Z`)) "None" true)
                (if (> _returnvalue_6 (`self.Trigger Depth`))
                  (`/Engine/EditorBlueprintResources/StandardMacros.DoOnce` false :!label _label
                    (:`Completed`
                      (`self.Pressed`))))))))
        (else
          (`SceneComponent.K2_SetWorldLocation` (`self.Button`) (+ (`SceneComponent.K2_GetComponentLocation` (`self.Plane`)) (* (`SceneComponent.GetUpVector` (`self.Plane`)) (`self.Button Height`))) false false)
          (`PrimitiveComponent.SetCollisionEnabled` (`self.Button`) "QueryAndPhysics"))))
    (:`then_3`
      (if (== (`SceneComponent.K2_GetComponentLocation` (`self.Button`)) _returnvalue_4 :`ErrorTolerance` (`self.Reset Point`))
        (`self.reset button`)))
    (:`then_4`
      (`SceneComponent.K2_SetWorldRotation` (`self.Button`) (`SceneComponent.K2_GetComponentRotation` (`self.Plane`)) false false))))

(event `reset button`
  (goto _label :!via `Reset`))

(event `Pressed`
  (if (`PrimitiveComponent.IsOverlappingComponent` (`self.Box`) (`/Game/Blueprint/BP_MotionController.FingerTip` (stale `self.Box.OnComponentBeginOverlap` _asbp_motion_controller)))
    (message `/Game/Blueprint/ButtonInterface.Button Pressed` (`self.Owning Actor`) (`self.Button Index`))
    (`/Engine/EditorBlueprintResources/StandardMacros.FlipFlop`
      (:`A`
        (`PrimitiveComponent.SetMaterial` (`self.Button`) 0 "/Game/Materials/brightgreen.brightgreen"))
      (:`B`
        (`PrimitiveComponent.SetMaterial` (`self.Button`) 0 "/Game/Materials/Light_4.Light_4")))))

(event `self.Box.OnComponentBeginOverlap`
  (params (OverlappedComponent :type "PrimitiveComponent Object Reference") (OtherActor :type "Actor Object Reference") (OtherComp :type "PrimitiveComponent Object Reference") (OtherBodyIndex :type Integer) (bFromSweep :type Boolean) (SweepResult :type "HitResult Structure (by ref)"))
  (bind _asbp_motion_controller (cast `/Game/Blueprint/BP_MotionController` OtherActor))
  (if (== OtherComp (`/Game/Blueprint/BP_MotionController.FingerTip` _asbp_motion_controller))
    (set `self.Overlapping Hand` _asbp_motion_controller)
    (set `self.Hand Overlapping?` true)
    (`PrimitiveComponent.SetSimulatePhysics` (`self.Button`) true)))

(event `self.Box.OnComponentEndOverlap`
  (params (OverlappedComponent :type "PrimitiveComponent Object Reference") (OtherActor :type "Actor Object Reference") (OtherComp :type "PrimitiveComponent Object Reference") (OtherBodyIndex :type Integer))
  (bind _asbp_motion_controller (cast `/Game/Blueprint/BP_MotionController` OtherActor))
  (if (== OtherComp (`/Game/Blueprint/BP_MotionController.FingerTip` _asbp_motion_controller))
    (set `self.Overlapping Hand` null)
    (set `self.Hand Overlapping?` false)
    (`PrimitiveComponent.SetSimulatePhysics` (`self.Button`) false)))

(fn `UserConstructionScript`)