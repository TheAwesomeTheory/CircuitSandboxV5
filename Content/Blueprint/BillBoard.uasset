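; BillBoard is an actor that floats a text sign on a cable above an owning actor.
; A low-poly text component, configured in the construction script, writes its text at BeginPlay, and the cable becomes visible shortly after.
; Each tick, the actor follows its owner at a height offset while stiffness-scaled spring forces keep the physics cube within cable length and push it away when too close.
; The cube also yaws toward the player camera.
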(event `self.ReceiveBeginPlay`
  (`/Game/LowPolyText/Blueprints/LowPolyTextComp.Write` (`self.LowPolyTextComp`))
  (`KismetSystemLibrary.Delay` 0.25)
  (`SceneComponent.SetVisibility` (`self.Cable`) true false))

(event `self.ReceiveTick`
  (params (DeltaSeconds :type "Float (single-precision)"))
  (`|ExecutionSequence`
    (:`then_0`
      (if (< (`self.cablelength`) (`KismetMathLibrary.VSize` (- (`SceneComponent.K2_GetComponentLocation` (`self.Cube`)) (`self.K2_GetActorLocation`))))
        (`PrimitiveComponent.AddForce` (`self.Cube`) (* (- (`self.K2_GetActorLocation`) (`SceneComponent.K2_GetComponentLocation` (`self.Cube`))) (`self.stiffness`)) "None" false)))
    (:`then_1`
      (if (< (`KismetMathLibrary.VSize` (- (`self.K2_GetActorLocation`) (`SceneComponent.K2_GetComponentLocation` (`self.Cube`)))) 30.0)
        (`PrimitiveComponent.AddForce` (`self.Cube`) (* (- (`SceneComponent.K2_GetComponentLocation` (`self.Cube`)) (`self.K2_GetActorLocation`)) (`self.stiffness`)) "None" false)
        (`KismetSystemLibrary.PrintString` "PUSHING")))
    (:`then_2`
      (`self.K2_SetActorLocation` (`KismetMathLibrary.MakeVector` (.x (`self.K2_GetActorLocation` (`self.Owning Actor`))) (.y (`self.K2_GetActorLocation` (`self.Owning Actor`))) (+ (.z (`self.K2_GetActorLocation` (`self.Owning Actor`))) (`self.Height Offset`))))
      (`SceneComponent.K2_SetWorldRotation` (`self.Cube`) (`KismetMathLibrary.MakeRotator` (.roll (`KismetMathLibrary.FindLookAtRotation` (`SceneComponent.K2_GetComponentLocation` (`self.Cube`)) (`PlayerCameraManager.GetCameraLocation` (`GameplayStatics.GetPlayerCameraManager` 0)))) 0.0 (+ (.yaw (`KismetMathLibrary.FindLookAtRotation` (`SceneComponent.K2_GetComponentLocation` (`self.Cube`)) (`PlayerCameraManager.GetCameraLocation` (`GameplayStatics.GetPlayerCameraManager` 0)))) 0.0)) false false))))

(fn `UserConstructionScript`
  (bind _parent_mesh_ref (`self.Parent Mesh Ref`))
  (bind _lowpolytextcomp (`self.LowPolyTextComp`))
  (set `/Game/LowPolyText/Blueprints/LowPolyTextComp.ParentMeshRef` _parent_mesh_ref (`self.LowPolyTextComp`))
  (set `/Game/LowPolyText/Blueprints/LowPolyTextComp.Text Data` (`self.Text Data`) _lowpolytextcomp)
  (set `/Game/LowPolyText/Blueprints/LowPolyTextComp.Parent Component` _parent_mesh_ref _lowpolytextcomp)
  (`SceneComponent.K2_SetRelativeLocation` (`self.Parent Mesh Ref`) (+ (`SceneComponent.RelativeLocation` (`self.Parent Mesh Ref`)) (`self.Text Offset`)) false false))